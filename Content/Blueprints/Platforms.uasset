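; Moving platform Blueprint that carries itself along a spline path while the third-person character is inside its trigger box.
; Box overlap plays the Platform_move timeline forward, and leaving the box reverses it back along the path.
; Each update scales the timeline value by spline length to set location and rotation, keeping pitch at zero so the platform follows only the spline's yaw and roll.
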(event OnComponentBeginOverlap(Box)
  (params (OverlappedComponent :type Primitive%20Component%20Object%20Reference) (OtherActor :type Actor%20Object%20Reference) (OtherComp :type Primitive%20Component%20Object%20Reference) (OtherBodyIndex :type Integer) (bFromSweep :type Boolean) (SweepResult :type Hit%20Result%20Structure%20%28by%20ref%29))
  (bind _spline (Variables|Default|GetSpline))
  (bind _platform (Variables|Default|GetPlatform))
  ;[1 1 1] Overlap
  (Utilities|Casting|CastToThirdPersonCharacter OtherActor)
  (bind _move_distance (Timeline|platform_move Play)
    (:Update
      (Transformation|SetWorldLocation _platform (Spline|GetLocationatDistanceAlongSpline _spline (* _move_distance (Spline|GetSplineLength _spline)) "World") false false)
      (Transformation|SetRelativeRotation _platform (Math|Rotator|MakeRotator (.roll (Spline|GetRotationatDistanceAlongSpline _spline (* _move_distance (Spline|GetSplineLength _spline)) "Local")) 0.0 (.yaw (Spline|GetRotationatDistanceAlongSpline _spline (* _move_distance (Spline|GetSplineLength _spline)) "Local"))) false false))))

(event OnComponentEndOverlap(Box)
  (params (OverlappedComponent :type Primitive%20Component%20Object%20Reference) (OtherActor :type Actor%20Object%20Reference) (OtherComp :type Primitive%20Component%20Object%20Reference) (OtherBodyIndex :type Integer))
  (bind _spline (Variables|Default|GetSpline))
  (bind _platform (Variables|Default|GetPlatform))
  ;[1 1 1] Overlap
  (Utilities|Casting|CastToThirdPersonCharacter OtherActor)
  (bind _move_distance (Timeline|platform_move Reverse)
    (:Update
      (Transformation|SetWorldLocation _platform (Spline|GetLocationatDistanceAlongSpline _spline (* _move_distance (Spline|GetSplineLength _spline)) "World") false false)
      (Transformation|SetRelativeRotation _platform (Math|Rotator|MakeRotator (.roll (Spline|GetRotationatDistanceAlongSpline _spline (* _move_distance (Spline|GetSplineLength _spline)) "Local")) 0.0 (.yaw (Spline|GetRotationatDistanceAlongSpline _spline (* _move_distance (Spline|GetSplineLength _spline)) "Local"))) false false))))

(event EventBeginPlay
  (bind _spline (Variables|Default|GetSpline))
  (bind _returnvalue (Spline|GetRotationatDistanceAlongSpline _spline 0.0 "Local"))
  ;[1 1 1] Begin_Play
  (Transformation|SetRelativeRotation (Variables|Default|GetPlatform) (Math|Rotator|MakeRotator (.roll _returnvalue) 0.0 (.yaw _returnvalue)) false false))

(fn ConstructionScript)