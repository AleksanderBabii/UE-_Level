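; Spike trap actor that damages combat characters when they hit its skeletal mesh.
; A combat character entering the box sets an IsTriggered flag, which a timer clears a few seconds later.
; Mesh hits send a damage message with hit data, gated by a DoOnce that resets after a short delay to act as a cooldown.
; The Deal_Damage event only checks player overlap with the box and does nothing further.
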(event OnComponentBeginOverlap(Box)
  (params (OverlappedComponent :type Primitive%20Component%20Object%20Reference) (OtherActor :type Actor%20Object%20Reference) (OtherComp :type Primitive%20Component%20Object%20Reference) (OtherBodyIndex :type Integer) (bFromSweep :type Boolean) (SweepResult :type Hit%20Result%20Structure%20%28by%20ref%29))
  (Utilities|Casting|CastToBP_CombatCharacter OtherActor)
  (if (not (Variables|Default|GetIsTriggered))
    (Variables|Default|SetIsTriggered true)
    (Utilities|Time|SetTimerbyEvent (delegate Custom|Reset) 3.5)))

(event OnComponentHit(SkeletalMesh)
  (params (HitComponent :type Primitive%20Component%20Object%20Reference) (OtherActor :type Actor%20Object%20Reference) (OtherComp :type Primitive%20Component%20Object%20Reference) (NormalImpulse :type Vector :default "0, 0, 0") (Hit :type Hit%20Result%20Structure%20%28by%20ref%29))
  (bind _asbp_combat_character (Utilities|Casting|CastToBP_CombatCharacter OtherActor))
  (Utilities|FlowControl|DoOnce false :!label _label
    (:Completed
      (Utilities|FlowControl|Sequence
        (:then_0
          (Class|ICanbeAttacked|TakeDamage(Message) _asbp_combat_character (Utilities|Struct|MakeF_HitData (Variables|Default|GetDamage) self)))
        (:then_1
          (Utilities|FlowControl|Delay 2.0)
          (goto _label Reset))))))

(event Custom|Reset
  (Variables|Default|SetIsTriggered false))

(event Custom|Deal_Damage
  (if (Collision|IsOverlappingActor (Variables|Default|GetBox) (Game|GetPlayerCharacter 0) :!class /Script/Engine.PrimitiveComponent)
    _))

(fn ConstructionScript)