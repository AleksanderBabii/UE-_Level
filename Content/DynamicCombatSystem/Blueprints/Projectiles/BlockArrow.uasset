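; BlockArrow is an arrow projectile that creates a TempPlatform where it strikes a non-character target.
; It overrides OnArrowHit, passing Character hits to the parent's logic.
; Other hits spawn the platform at the impact point with its X axis along the surface normal, attached to the hit actor and component with world transform kept.
; The arrow then destroys itself and returns false.
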(event EventBeginPlay
  (|CallParentFunction) ; This node is disabled and will not be called.\nDrag off pins to build functionality.
)

(event Collision|EventActorBeginOverlap
  (params (OtherActor :type Actor%20Object%20Reference)))

(event EventTick
  (params (DeltaSeconds :type Float%20%28single-precision%29)))

(fn ConstructionScript
  (|CallParentFunction))

(fn OnArrowHit
  (params (Hit :type Hit%20Result%20Structure%20%28by%20ref%29))
  (bind (_bblockinghit _binitialoverlap _time _distance _location _impactpoint _normal _impactnormal _physmat _hitactor _hitcomponent) (Collision|BreakHitResult Hit))
  (Utilities|Casting|CastToCharacter _hitactor
    (:then
      (bind _dummy (|CallParentFunction Hit))
      (return _dummy))
    (:CastFailed
      (bind _returnvalue (Game|SpawnActorfromClass "/Game/LevelDesignMechanics/TempPlatform.TempPlatform_C" (Math|Transform|MakeTransform _location (Math|Conversions|RotationFromXVector _impactnormal) "1,1,1") "Undefined" 0 0))
      (Transformation|AttachActorToActor _returnvalue _hitactor "None" "KeepWorld" "KeepWorld" "KeepWorld" true)
      (Transformation|AttachComponentToComponent _returnvalue _hitcomponent "None" "KeepWorld" "KeepWorld" "KeepWorld" true)
      (Actor|DestroyActor)
      (return false))))