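; Arrow projectile variant in the Dynamic Combat System that freezes compatible actors it hits.
; Its OnArrowHit override checks the hit actor for ImpulseInterface, calling Freeze directly on a MovingPlatform and FreezeMessage on any other implementer.
; The parent hit logic runs only after a freeze, so hits on actors without the interface skip it.
; The event graph and construction script add no behavior of their own.
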(event EventBeginPlay
  (|CallParentFunction) ; This node is disabled and will not be called.\nDrag off pins to build functionality.
)

(event Collision|EventActorBeginOverlap
  (params (OtherActor :type Actor%20Object%20Reference)))

(event EventTick
  (params (DeltaSeconds :type Float%20%28single-precision%29)))

(fn ConstructionScript
  (|CallParentFunction))

(fn OnArrowHit
  (params (Hit :type Hit%20Result%20Structure%20%28by%20ref%29))
  (bind _hitactor (Collision|BreakHitResult Hit))
  (if (Utilities|DoesObjectImplementInterface _hitactor "/Game/LevelDesignMechanics/ImpulseInterface.ImpulseInterface_C")
    (bind _asmoving_platform (Utilities|Casting|CastToMovingPlatform _hitactor)
      (:then
        (Default|Freeze _asmoving_platform))
      (:CastFailed
        (Class|ImpulseInterface|Freeze(Message) _hitactor)))
    (bind _dummy (|CallParentFunction Hit))
    (return _dummy)))